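; Charged projectile that deals double the player's equipped weapon damage to a MasterEnemy it hits.
; On movement activation it takes a random rotation with homing off, while a timeline drives homing acceleration and enables homing when finished.
; A looping timer runs short forward object traces; any hit destroys the projectile, with enemy hits also applying damage and a fire effect.
; Unspent projectiles expire after a fixed delay.
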(event `self.ProjectileMovement.OnComponentActivated`
  (params (Component :type "ActorComponent Object Reference") (bReset :type Boolean))
  (bind _returnvalue (`KismetMathLibrary.RandomFloatInRange` 0.0 180.0))
  (bind _projectilemovement (`self.ProjectileMovement`))
  (`KismetSystemLibrary.K2_SetTimerDelegate` (delegate `TracingForDamage`) 0.01 true)
  (bind _astest_3rd_person_controller (cast `/Game/CustomBlueprints/Test3rdPersonController` (`GameplayStatics.GetPlayerCharacter` 0)))
  (bind _output_get (set `self.CharacterREf` _astest_3rd_person_controller))
  (`|ExecutionSequence`
    (:`then_0`
      (bind (_direction _speedalpha) (`Timeline|Timeline_0` :!via `PlayFromStart`)
        (:`Update`
          (set `ProjectileMovementComponent.HomingAccelerationMagnitude` _speedalpha _projectilemovement))
        (:`Finished`
          (set `ProjectileMovementComponent.bIsHomingProjectile` true (`self.ProjectileMovement`)))))
    (:`then_1`
      (`self.K2_SetActorRotation` (`KismetMathLibrary.MakeRotator` (+ 0.0 _returnvalue) (+ 0.0 _returnvalue) (+ 0.0 (`KismetMathLibrary.RandomFloatInRange` 1.0 360.0))))
      (set `ProjectileMovementComponent.bIsHomingProjectile` false _projectilemovement)
      (set `self.ProjectileDamage` (* (`/Game/VoxelAssets/Other/BasicSword.Damage` (`/Game/CustomBlueprints/Test3rdPersonController.EquippedWeapon` _output_get)) 2.0))
      (set `ProjectileMovementComponent.MaxSpeed` 1000.0 _projectilemovement)
      (`KismetSystemLibrary.Delay` 15.0)
      (`/Engine/EditorBlueprintResources/StandardMacros.IsValid` self
        (:`Is Valid`
          (`self.K2_DestroyActor`))))))

(event `TracingForDamage`
  (bind _sphere (`self.Sphere`))
  (bind _returnvalue (`SceneComponent.K2_GetComponentLocation` _sphere))
  (bind (_outhit _returnvalue_2) (`KismetSystemLibrary.LineTraceSingleForObjects` _returnvalue (+ _returnvalue (* (`SceneComponent.GetForwardVector` _sphere) 10.0)) (`|MakeArray` "ObjectTypeQuery3" "ObjectTypeQuery1" :!type "EObjectTypeQuery Enum") false (`|MakeArray` (`self.CharacterREf`) :!type "Actor Object Reference") "ForDuration" true (struct :`R` 1.0 :`A` 1.0) (struct :`G` 1.0 :`A` 1.0) 0.5))
  (if _returnvalue_2
    (bind _outactors (`GameplayStatics.GetAllActorsOfClass` "/Game/CustomBlueprints/MasterEnemy.MasterEnemy_C"))
    (for _array_element _outactors
      (bind (_bblockinghit _binitialoverlap _time _distance _location _impactpoint _normal _impactnormal _physmat _hitactor) (`GameplayStatics.BreakHitResult` _outhit))
      (if (!= _array_element _hitactor)
        (`self.K2_DestroyActor`)
        (else
          (set `self.DamagedEnemy` _array_element)
          (if (and (== _array_element _hitactor) (not (`KismetArrayLibrary.Array_Contains` (`self.AlreadyDamagedEnemy`) (`self.DamagedEnemy`))))
            (`KismetArrayLibrary.Array_Add` (`self.AlreadyDamagedEnemy`) (`self.DamagedEnemy`))
            (`/Game/CustomBlueprints/DamageInterface.DealingDamage` (`self.DamagedEnemy`) (`self.ProjectileDamage`) null false)
            (`GameplayStatics.SpawnEmitterAtLocation` "/Game/AdvancedMagicFX12/particles/P_ky_hit_fire.P_ky_hit_fire" _impactpoint (struct) (0.5 0.5 0.5))
            (`self.K2_DestroyActor`)))))))

(fn `UserConstructionScript`)