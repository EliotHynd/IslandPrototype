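; HUD Blueprint that draws a small centred texture, likely a crosshair, and an orange stamina wheel near the top-left.
; Each DrawHUD call creates a new dynamic material instance from StaminaWheel and feeds it the Test3rdPersonController's CurrentEnergy to MaxEnergy ratio.
; An authority switch picks the character source: player index 0 on authority, index 1 on remote.
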(event `self.ReceiveDrawHUD`
  (params (SizeX :type Integer) (SizeY :type Integer))
  (bind _astest_3rd_person_controller (cast `/Game/CustomBlueprints/Test3rdPersonController` (`GameplayStatics.GetPlayerCharacter` 1) :!pure true))
  (bind (_astest_3rd_person_controller_2 _bsuccess) (cast `/Game/CustomBlueprints/Test3rdPersonController` (`GameplayStatics.GetPlayerCharacter` 0) :!pure true))
  (`self.DrawTexture` null (`KismetMathLibrary.Conv_IntToDouble` (- (/ SizeX 2) 3)) (`KismetMathLibrary.Conv_IntToDouble` (- (/ SizeY 2) 3)))
  (bind _returnvalue (`KismetMaterialLibrary.CreateDynamicMaterialInstance` "/Game/Materials/StaminaWheel.StaminaWheel"))
  (`MaterialInstanceDynamic.SetVectorParameterValue` _returnvalue "Colour" (struct :`R` 1.0 :`G` 0.654189 :`A` 1.0))
  (`/Engine/EditorBlueprintResources/ActorMacros.Switch Has Authority`
    (:`Authority`
      (if _bsuccess
        (`MaterialInstanceDynamic.SetScalarParameterValue` _returnvalue "Decimal" (/ (`/Game/CustomBlueprints/Test3rdPersonController.CurrentEnergy` _astest_3rd_person_controller_2) (`/Game/CustomBlueprints/Test3rdPersonController.MaxEnergy` _astest_3rd_person_controller_2)))
        (`self.DrawMaterialSimple` _returnvalue 100.0 100.0 100.0 100.0)))
    (:`Remote`
      (`MaterialInstanceDynamic.SetScalarParameterValue` _returnvalue "Decimal" (/ (`/Game/CustomBlueprints/Test3rdPersonController.CurrentEnergy` _astest_3rd_person_controller) (`/Game/CustomBlueprints/Test3rdPersonController.MaxEnergy` _astest_3rd_person_controller)))
      (`self.DrawMaterialSimple` _returnvalue 100.0 100.0 100.0 100.0))))

(fn `UserConstructionScript`)