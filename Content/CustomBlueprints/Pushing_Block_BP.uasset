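; Pushable block actor that detects which of its four sides the Test3rdPersonController player is touching.
; Each side's overlap events set or clear a matching boolean flag.
; Sides 2–4 also write a fixed axis-aligned push direction onto the player.
; Side 1 looks unfinished: it sets no direction, instead calling a MoveComponentTo with no component or target location supplied, then printing a debug string.
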(event `self.Side 1.OnComponentBeginOverlap`
  (params (OverlappedComponent :type "PrimitiveComponent Object Reference") (OtherActor :type "Actor Object Reference") (OtherComp :type "PrimitiveComponent Object Reference") (OtherBodyIndex :type Integer) (bFromSweep :type Boolean) (SweepResult :type "HitResult Structure (by ref)"))
  (bind _astest_3rd_person_controller (cast `/Game/CustomBlueprints/Test3rdPersonController` OtherActor))
  (set `self.Side_1` true)
  (`KismetSystemLibrary.MoveComponentTo` null (0.0 0.0 0.0) (struct) false false 1.0)
  (`KismetSystemLibrary.PrintString` "Yas"))

(event `self.Side 1.OnComponentEndOverlap`
  (params (OverlappedComponent :type "PrimitiveComponent Object Reference") (OtherActor :type "Actor Object Reference") (OtherComp :type "PrimitiveComponent Object Reference") (OtherBodyIndex :type Integer))
  (cast `/Game/CustomBlueprints/Test3rdPersonController` OtherActor)
  (set `self.Side_1` false))

(event `self.Side 2.OnComponentBeginOverlap`
  (params (OverlappedComponent :type "PrimitiveComponent Object Reference") (OtherActor :type "Actor Object Reference") (OtherComp :type "PrimitiveComponent Object Reference") (OtherBodyIndex :type Integer) (bFromSweep :type Boolean) (SweepResult :type "HitResult Structure (by ref)"))
  (bind _astest_3rd_person_controller (cast `/Game/CustomBlueprints/Test3rdPersonController` OtherActor))
  (set `self.Side_2` true)
  (set `/Game/CustomBlueprints/Test3rdPersonController.SetPushDirectoin` (0.0 -1.0 0.0) _astest_3rd_person_controller))

(event `self.Side 2.OnComponentEndOverlap`
  (params (OverlappedComponent :type "PrimitiveComponent Object Reference") (OtherActor :type "Actor Object Reference") (OtherComp :type "PrimitiveComponent Object Reference") (OtherBodyIndex :type Integer))
  (cast `/Game/CustomBlueprints/Test3rdPersonController` OtherActor)
  (set `self.Side_2` false))

(event `self.Side 3.OnComponentBeginOverlap`
  (params (OverlappedComponent :type "PrimitiveComponent Object Reference") (OtherActor :type "Actor Object Reference") (OtherComp :type "PrimitiveComponent Object Reference") (OtherBodyIndex :type Integer) (bFromSweep :type Boolean) (SweepResult :type "HitResult Structure (by ref)"))
  (bind _astest_3rd_person_controller (cast `/Game/CustomBlueprints/Test3rdPersonController` OtherActor))
  (set `self.Side_3` true)
  (set `/Game/CustomBlueprints/Test3rdPersonController.SetPushDirectoin` (0.0 1.0 0.0) _astest_3rd_person_controller))

(event `self.Side 3.OnComponentEndOverlap`
  (params (OverlappedComponent :type "PrimitiveComponent Object Reference") (OtherActor :type "Actor Object Reference") (OtherComp :type "PrimitiveComponent Object Reference") (OtherBodyIndex :type Integer))
  (cast `/Game/CustomBlueprints/Test3rdPersonController` OtherActor)
  (set `self.Side_3` false))

(event `self.Side 4.OnComponentBeginOverlap`
  (params (OverlappedComponent :type "PrimitiveComponent Object Reference") (OtherActor :type "Actor Object Reference") (OtherComp :type "PrimitiveComponent Object Reference") (OtherBodyIndex :type Integer) (bFromSweep :type Boolean) (SweepResult :type "HitResult Structure (by ref)"))
  (bind _astest_3rd_person_controller (cast `/Game/CustomBlueprints/Test3rdPersonController` OtherActor))
  (set `self.Side_4` true)
  (set `/Game/CustomBlueprints/Test3rdPersonController.SetPushDirectoin` (1.0 0.0 0.0) _astest_3rd_person_controller))

(event `self.Side 4.OnComponentEndOverlap`
  (params (OverlappedComponent :type "PrimitiveComponent Object Reference") (OtherActor :type "Actor Object Reference") (OtherComp :type "PrimitiveComponent Object Reference") (OtherBodyIndex :type Integer))
  (cast `/Game/CustomBlueprints/Test3rdPersonController` OtherActor)
  (set `self.Side_4` false))

(fn `UserConstructionScript`)